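; Player State Blueprint that exposes the Steam player's identity for display.
; SetPlayerName writes the online nickname into a supplied text object, while PlayerName returns the unique net ID as text rather than the nickname.
; Both resolve the ID through player controller 0 instead of the state's own owner, and PlayerState simply returns a self reference.
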(event EventSetPlayerName
  (params (Text :type Text%20Block%20Object%20Reference))
  (Rendering|Components|TextRender|SetText Text (Utilities|Text|ToText(String) (Class|AdvancedIdentityLibrary|GetPlayerNickname (Class|AdvancedSessionsLibrary|GetUniqueNetID (Game|GetPlayerController 0))))))

(fn ConstructionScript)

(fn PlayerName
  (return (Utilities|Text|ToText(String) (Class|AdvancedSessionsLibrary|UniqueNetIdtoString (Class|AdvancedSessionsLibrary|GetUniqueNetID (Game|GetPlayerController 0))))))

(fn PlayerState
  (return self))